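; Turret actor that tracks the player pawn with its top and line-traces toward it once roughly aimed.
; Each Tick, a dot product against the top's forward vector tests for a wide view cone, inside which yaw eases toward the player using Atan2 and a frame-time-scaled Lerp.
; A second, much tighter dot threshold triggers a debug-drawn multi line trace from the Arrow component; the hit results are unused.
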(event `self.ReceiveTick`
  (params (DeltaSeconds :type "Float (single-precision)"))
  (bind _turrettop (`self.TurretTop`))
  (bind _arrow (`self.Arrow`))
  (bind (_returnvalue_roll _returnvalue_pitch _returnvalue_yaw) (`KismetMathLibrary.BreakRotator` (`SceneComponent.K2_GetComponentRotation` _turrettop)))
  (bind (_returnvalue_x _returnvalue_y) (`KismetMathLibrary.BreakVector` (`KismetMathLibrary.Normal` (- (`self.K2_GetActorLocation` (`GameplayStatics.GetPlayerPawn` 0)) (`SceneComponent.K2_GetComponentLocation` (`self.TurretTop`))))))
  (bind _returnvalue (`KismetMathLibrary.Dot_VectorVector` (`KismetMathLibrary.Normal` (`SceneComponent.GetForwardVector` (`self.TurretTop`))) (`KismetMathLibrary.Normal` (- (`self.K2_GetActorLocation` (`GameplayStatics.GetPlayerPawn` 0)) (`self.K2_GetActorLocation`)))))
  (set `self.Delta Seconds` DeltaSeconds)
  (if (>= _returnvalue 0.7)
    (`SceneComponent.K2_SetWorldRotation` _turrettop (`KismetMathLibrary.MakeRotator` 0.0 0.0 (`KismetMathLibrary.Lerp` _returnvalue_yaw (`KismetMathLibrary.DegAtan2` _returnvalue_y _returnvalue_x) (* (`self.Delta Seconds`) 5.0))) false false)
    (if (>= _returnvalue 0.989)
      (`KismetSystemLibrary.LineTraceMulti` :`Start` (`SceneComponent.K2_GetComponentLocation` _arrow) :`End` (+ (`SceneComponent.K2_GetComponentLocation` _arrow) (* (`SceneComponent.GetForwardVector` _arrow) 1000.0)) :`TraceChannel` "TraceTypeQuery1" :`bTraceComplex` true :`DrawDebugType` "ForDuration"))))

(fn `UserConstructionScript`)